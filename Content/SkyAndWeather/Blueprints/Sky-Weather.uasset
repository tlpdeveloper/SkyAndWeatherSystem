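; Sky actor that runs a looping 24-hour day and night cycle with a Sun and a Moon light.
; Tick advances Time at a rate set by DayLenght and wraps it to zero near midnight.
; Time maps linearly to each light's pitch, keeping Sun and Moon half a turn apart.
; The construction script also applies the rotations, plus fixed day and night intensities, so edits preview in the editor.
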(event `self.ReceiveTick`
  (params (DeltaSeconds :type "Float (single-precision)"))
  (`self.Update Time ` DeltaSeconds)
  (`self.Update Sun And Moon`))

(fn `Get Moon Rotation`
  (returns (ReturnValue :type "Float (double-precision)"))
  (return (+ (* (/ (`self.Time`) 24.0) 360.0) -90.0)))

(fn `Get Sun Rotation`
  (returns (ReturnValue :type "Float (double-precision)"))
  (return (+ (* (/ (`self.Time`) 24.0) 360.0) 90.0)))

(fn `Pre Update`
  (`LightComponent.SetIntensity` (`self.Sun`) (`self.Day Brightness`))
  (`LightComponent.SetIntensity` (`self.Moon`) (`self.Night Brightness`)))

(fn `Update Sun And Moon`
  (`SceneComponent.K2_SetRelativeRotation` (`self.Sun`) (`KismetMathLibrary.MakeRotator` 0.0 (`self.Get Sun Rotation`)) false false)
  (`SceneComponent.K2_SetRelativeRotation` (`self.Moon`) (`KismetMathLibrary.MakeRotator` 0.0 (`self.Get Moon Rotation`)) false false))

(fn `Update Time `
  (params (DeltaTime :type "Float (double-precision)"))
  (if (>= (`self.Time`) 23.99)
    (set `self.Time` 0.0)
    (else
      (set `self.Time` (+ (`self.Time`) (/ DeltaTime (`self.DayLenght`))))))
  (return))

(fn `UserConstructionScript`
  (`self.Update Sun And Moon`)
  (`self.Pre Update`))